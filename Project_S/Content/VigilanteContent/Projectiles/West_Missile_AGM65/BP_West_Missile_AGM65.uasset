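; Blueprint for the Western AGM-65 missile projectile, providing visual control of its engine effect and four fins.
; BeginPlay caches the skeletal mesh's BPA_West_Missile_AGM65 anim instance.
; An engine-state event toggles the thruster FX with a reset, while per-fin events remap normalized, clamped inputs to deflection angles and write them to the anim instance.
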(event `self.ReceiveBeginPlay`
  (bind _asbpa_west_missile_agm65 (cast `/Game/VigilanteContent/Projectiles/West_Missile_AGM65/BPA_West_Missile_AGM65` (`SkeletalMeshComponent.GetAnimInstance` (`self.SkeletalMesh`))))
  (set `self.AnimInstance` _asbpa_west_missile_agm65))

(event `SetEngineState`
  (params (bEngineActive :type Boolean))
  ;[1 1 1] Set engine state
  (`ActorComponent.SetActive` (`self.ThrusterFX`) bEngineActive true))

(event `SetFin1Angle`
  (params (Angle :type "Float (double-precision)"))
  (set `/Game/VigilanteContent/Projectiles/West_Missile_AGM65/BPA_West_Missile_AGM65.Fin1Angle` (`KismetMathLibrary.MapRangeClamped` Angle -1.0 1.0 -45.0 45.0) (`self.AnimInstance`)))

(event `SetFin2Angle`
  (params (Angle :type "Float (double-precision)"))
  (set `/Game/VigilanteContent/Projectiles/West_Missile_AGM65/BPA_West_Missile_AGM65.Fin2Angle` (`KismetMathLibrary.MapRangeClamped` Angle -1.0 1.0 -45.0 45.0) (`self.AnimInstance`)))

(event `SetFin3Angle`
  (params (Angle :type "Float (double-precision)"))
  (set `/Game/VigilanteContent/Projectiles/West_Missile_AGM65/BPA_West_Missile_AGM65.Fin3Angle` (`KismetMathLibrary.MapRangeClamped` Angle -1.0 1.0 -45.0 45.0) (`self.AnimInstance`)))

(event `SetFin4Angle`
  (params (Angle :type "Float (double-precision)"))
  (set `/Game/VigilanteContent/Projectiles/West_Missile_AGM65/BPA_West_Missile_AGM65.Fin4Angle` (`KismetMathLibrary.MapRangeClamped` Angle -1.0 1.0 -45.0 45.0) (`self.AnimInstance`)))

(fn `UserConstructionScript`)